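; AI controller for the Nemo NPC that sends it from coin to coin and removes them.
; On BeginPlay it gathers every BP_Coin whose location projects onto the navmesh into a list, in found order rather than by distance.
; GoToNextCoin moves to the first entry, and RemoveCoin destroys that coin, then moves on to the next.
; Nothing in this graph starts the first move or calls RemoveCoin.
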(event `self.ReceiveBeginPlay`
  (`self.InitCoin`))

(event `InitCoin`
  (bind _outactors (`GameplayStatics.GetAllActorsOfClass` "/Game/Elvyn/Blueprints/BP_Coin.BP_Coin_C"))
  (for _array_element _outactors
    (if (`.ReturnValue` (`NavigationSystemV1.K2_ProjectPointToNavigation` (`self.K2_GetActorLocation` _array_element)))
      (`KismetArrayLibrary.Array_AddUnique` (`self.coinList`) _array_element))))

(event `GoToNextCoin`
  (bind _output (`|GetArrayItem` (`self.coinList`)))
  (if (`KismetSystemLibrary.IsValid` _output)
    (`self.MoveToActor` _output -1.0 true true true null)))

(event `RemoveCoin`
  (bind _output (`|GetArrayItem` (`self.coinList`)))
  (if (`KismetSystemLibrary.IsValid` _output)
    (`self.K2_DestroyActor` _output)
    (`KismetArrayLibrary.Array_Remove` (`self.coinList`))
    (`self.GoToNextCoin`)))

(fn `UserConstructionScript`)