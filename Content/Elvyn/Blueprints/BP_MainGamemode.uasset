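; BP_MainGamemode is the game mode that tracks the player's checkpoint and handles game over.
; On BeginPlay it caches the FirstPersonCharacter and enables input for player controller 0.
; UpdateCheckpoint stores the new checkpoint as LastCheckPoint and prints it for debugging, though no respawn logic here reads it.
; GameOver prints a message, waits briefly, then opens the ElvynSalle level.
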(event `self.ReceiveBeginPlay`
  ;[1 1 1] Gets the player character
  (bind _returnvalue (`GameplayStatics.GetActorOfClass` "/Game/FirstPersonBP/Blueprints/FirstPersonCharacter.FirstPersonCharacter_C"))
  (set `self.CharacterPlayer` _returnvalue)
  (`self.EnableInput` (`GameplayStatics.GetPlayerController` 0)))

(event `Update Checkpoint`
  (params (newCheckPoint :type "Transform Structure"))
  ;[1 1 1] Update and prints location of checkpoint
  (bind _output_get (set `self.lastCheckPoint` newCheckPoint))
  (`KismetSystemLibrary.PrintString` (`KismetStringLibrary.Conv_TransformToString` _output_get)))

(event `GameOver`
  ;[1 1 1] Prints Gameover and opens the level
  (`KismetSystemLibrary.PrintString` "Game over")
  (`KismetSystemLibrary.Delay` 2.0)
  (`GameplayStatics.OpenLevelBySoftObjectPtr` "/Game/Elvyn/Level/ElvynSalle.ElvynSalle"))

(fn `UserConstructionScript`)