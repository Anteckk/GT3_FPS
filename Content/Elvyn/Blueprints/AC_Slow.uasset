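; AC_Slow is a timed slow-effect actor component that works on an NPC_Nemo owner.
; On BeginPlay it divides the NPC's max walk speed by its SlowFactor and sets BodyColor to red on a dynamic material instance of its mesh.
; After a five-second delay it multiplies the speed back, changes the NPC's state, calls StateManager and destroys itself, without resetting the color itself.
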(event `self.ReceiveBeginPlay`
  (bind _asnpc_nemo (cast `/Game/Elvyn/Blueprints/NPC_Nemo` (`self.GetOwner`)))
  (`KismetSystemLibrary.PrintString` "AC_Slow" true true (struct :`R` 0.65546 :`G` 1.0 :`A` 1.0) 5.0)
  (bind _charactermovement (`Character.CharacterMovement` _asnpc_nemo))
  (bind _maxwalkspeed (`CharacterMovementComponent.MaxWalkSpeed` _charactermovement))
  (bind _slowfactor (`/Game/Elvyn/Blueprints/NPC_Nemo.SlowFactor` _asnpc_nemo))
  (set `CharacterMovementComponent.MaxWalkSpeed` (/ _maxwalkspeed _slowfactor) _charactermovement)
  (bind _returnvalue (`Actor.GetComponentByClass` _asnpc_nemo "/Script/Engine.SkeletalMeshComponent"))
  (bind _returnvalue_2 (`PrimitiveComponent.CreateDynamicMaterialInstance` _returnvalue 0 (`PrimitiveComponent.GetMaterial` _returnvalue 0) "None"))
  (`MaterialInstanceDynamic.SetVectorParameterValue` _returnvalue_2 "BodyColor" (struct :`R` 1.0 :`A` 1.0))
  (`KismetSystemLibrary.Delay` 5.0)
  (set `CharacterMovementComponent.MaxWalkSpeed` (* _maxwalkspeed _slowfactor) _charactermovement)
  (set `/Game/Elvyn/Blueprints/NPC_Nemo.State` "NewEnumerator4" _asnpc_nemo)
  (`/Game/Elvyn/Blueprints/NPC_Nemo.StateManager` _asnpc_nemo)
  (`self.K2_DestroyComponent`))