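; BP_RespawnZone is a trigger volume that sends the player back to the last checkpoint and costs them a life.
; When the player pawn overlaps its Box, it reads LastCheckPoint from BP_MainGameMode, teleports the pawn to that location and restores the control rotation.
; It then calls LoseLife on the FirstPersonCharacter.
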(event `self.Box.OnComponentBeginOverlap`
  (params (OverlappedComponent :type "PrimitiveComponent Object Reference") (OtherActor :type "Actor Object Reference") (OtherComp :type "PrimitiveComponent Object Reference") (OtherBodyIndex :type Integer) (bFromSweep :type Boolean) (SweepResult :type "HitResult Structure (by ref)"))
  (bind _returnvalue (`GameplayStatics.GetPlayerPawn` 0))
  ;[1 1 1] tp player to respawn point and looses a life
  (if (== OtherActor _returnvalue)
    (bind _asbp_main_game_mode (cast `/Game/Elvyn/Blueprints/BP_MainGamemode` (`GameplayStatics.GetGameMode`)))
    (bind (_lastcheckpoint_location _lastcheckpoint_rotation) (`KismetMathLibrary.BreakTransform` (`/Game/Elvyn/Blueprints/BP_MainGamemode.lastCheckPoint` _asbp_main_game_mode)))
    (`self.K2_SetActorLocation` _returnvalue _lastcheckpoint_location false true)
    (`Controller.SetControlRotation` (`GameplayStatics.GetPlayerController` 0) _lastcheckpoint_rotation)
    (bind _asfirst_person_character (cast `/Game/FirstPersonBP/Blueprints/FirstPersonCharacter` _returnvalue))
    (`/Game/FirstPersonBP/Blueprints/FirstPersonCharacter.LoseLife` _asfirst_person_character)))

(fn `UserConstructionScript`)