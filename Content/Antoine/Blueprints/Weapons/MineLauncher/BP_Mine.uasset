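; Mine actor for the mine launcher that destroys itself five seconds after spawning.
; CollisionFloor stops the mine's physics when it overlaps a platform Blueprint of one specific class.
; CollisionEnemy maintains a Hostiles list of NPC_Nemo actors, adding those tagged Enemy on overlap and removing them on exit.
; Radial damage and body-color tinting logic is disconnected, so the mine currently deals no damage.
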(event `self.ReceiveBeginPlay`
  (`KismetSystemLibrary.Delay` 5.0)
  (`self.K2_DestroyActor`))

(event `self.CollisionFloor.OnComponentBeginOverlap`
  (params (OverlappedComponent :type "PrimitiveComponent Object Reference") (OtherActor :type "Actor Object Reference") (OtherComp :type "PrimitiveComponent Object Reference") (OtherBodyIndex :type Integer) (bFromSweep :type Boolean) (SweepResult :type "HitResult Structure (by ref)"))
  (if (== (`GameplayStatics.GetObjectClass` OtherActor) "/Game/Antoine/Blueprints/PL_16m_Platform_Blueprint.PL_16m_Platform_Blueprint_C")
    (`PrimitiveComponent.SetSimulatePhysics` (`self.Mine`) false)))

(event `self.CollisionEnemy.OnComponentBeginOverlap`
  (params (OverlappedComponent :type "PrimitiveComponent Object Reference") (OtherActor :type "Actor Object Reference") (OtherComp :type "PrimitiveComponent Object Reference") (OtherBodyIndex :type Integer) (bFromSweep :type Boolean) (SweepResult :type "HitResult Structure (by ref)"))
  (if (`self.ActorHasTag` OtherActor "Enemy")
    (bind _asnpc_nemo (cast `/Game/Elvyn/Blueprints/NPC_Nemo` OtherActor))
    (`KismetArrayLibrary.Array_AddUnique` (`self.Hostiles`) _asnpc_nemo)))

(event `self.CollisionEnemy.OnComponentEndOverlap`
  (params (OverlappedComponent :type "PrimitiveComponent Object Reference") (OtherActor :type "Actor Object Reference") (OtherComp :type "PrimitiveComponent Object Reference") (OtherBodyIndex :type Integer))
  (bind _asnpc_nemo (cast `/Game/Elvyn/Blueprints/NPC_Nemo` OtherActor))
  (`KismetArrayLibrary.Array_RemoveItem` (`self.Hostiles`) _asnpc_nemo))

(event `self.ReceiveHit`
  (params (MyComp :type "PrimitiveComponent Object Reference") (Other :type "Actor Object Reference") (OtherComp :type "PrimitiveComponent Object Reference") (bSelfMoved :type Boolean) (HitLocation :type "Vector Structure") (HitNormal :type "Vector Structure") (NormalImpulse :type "Vector Structure") (Hit :type "HitResult Structure (by ref)")))

(fn `UserConstructionScript`)