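; Actor component that periodically changes its owning character's walk speed and body color for a limited time.
; On BeginPlay it creates a dynamic material on the skeletal mesh and starts a looping timer at twice EffectDuration.
; Each tick of that timer divides MaxWalkSpeed by AccelerationFactor and applies AccelerationColor.
; After an EffectDuration delay it multiplies the speed back and restores DefaultColor, alternating equal affected and normal phases.
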(event `self.ReceiveBeginPlay`
  (bind _returnvalue (`Actor.GetComponentByClass` (`self.GetOwner`) "/Script/Engine.SkeletalMeshComponent"))
  (bind _returnvalue_2 (`PrimitiveComponent.CreateDynamicMaterialInstance` _returnvalue 0 (`PrimitiveComponent.GetMaterial` _returnvalue 0) "None"))
  (bind _output_get (set `self.MI_CharacterBody` _returnvalue_2))
  (`MaterialInstanceDynamic.SetVectorParameterValue` _output_get "Bodycolor" (`self.DefaultColor`))
  (`KismetSystemLibrary.K2_SetTimerDelegate` (delegate `Slow`) (* 2 (`self.EffectDuration`)) true))

(event `Slow`
  (bind _accelerationfactor (`self.AccelerationFactor`))
  (bind _mi_characterbody (`self.MI_CharacterBody`))
  (bind _returnvalue (`Actor.GetComponentByClass` (`self.GetOwner`) "/Script/Engine.CharacterMovementComponent"))
  (bind _maxwalkspeed (`CharacterMovementComponent.MaxWalkSpeed` _returnvalue))
  (set `CharacterMovementComponent.MaxWalkSpeed` (/ _maxwalkspeed _accelerationfactor) _returnvalue)
  (`MaterialInstanceDynamic.SetVectorParameterValue` _mi_characterbody "BodyColor" (`self.AccerelationColor`))
  (`KismetSystemLibrary.Delay` (`self.EffectDuration`))
  (set `CharacterMovementComponent.MaxWalkSpeed` (* _accelerationfactor _maxwalkspeed) _returnvalue)
  (`MaterialInstanceDynamic.SetVectorParameterValue` _mi_characterbody "BodyColor" (`self.DefaultColor`)))