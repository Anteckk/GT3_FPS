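; BP_BA-RPP99 is a player weapon with water and ice fire modes, toggled with E and active only while its weapon slot is equipped.
; Water mode launches an impulse-driven BP_WaterDrop from an arrow component.
; Ice mode affects NPC_Nemo targets tracked by a cylinder overlap zone, icing wet ones and slowing others through their StateManager.
; The Shoot event has no trigger in this graph, and debug prints report modes and effects.
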(event `self.ReceiveBeginPlay`
  ;[1 1 1] enabling input and seting auto fire rate
  (`self.EnableInput` (`GameplayStatics.GetPlayerController` 0)))

(event `self.Shoot`
  (bind _return_value (`self.Weapon Check`))
  (if _return_value
    ;[1 1 1] check fire mode
    (if (`self.FireMode`)
      ;[1 1 1] ice mode
      (`KismetSystemLibrary.PrintString` "ICE" true true (struct :`G` 1.0 :`B` 0.98264 :`A` 1.0))
      (for _array_element (`self.Hostiles`)
        (if (`/Game/Elvyn/Blueprints/NPC_Nemo.Wet` _array_element)
          (set `/Game/Elvyn/Blueprints/NPC_Nemo.Iced` true _array_element)
          (set `/Game/Elvyn/Blueprints/NPC_Nemo.State` "NewEnumerator2" _array_element)
          (`/Game/Elvyn/Blueprints/NPC_Nemo.StateManager` _array_element)
          (`KismetSystemLibrary.PrintString` "Iced" true true (struct :`G` 0.782177 :`B` 1.0 :`A` 1.0))
          (else
            (set `/Game/Elvyn/Blueprints/NPC_Nemo.Slowed` true _array_element)
            (set `/Game/Elvyn/Blueprints/NPC_Nemo.State` "NewEnumerator1" _array_element)
            (`/Game/Elvyn/Blueprints/NPC_Nemo.StateManager` _array_element)
            (`KismetSystemLibrary.PrintString` "Slowed" true true (struct :`R` 0.973217 :`B` 1.0 :`A` 1.0)))))
      (else
        ;[1 1 1] water mode
        (`KismetSystemLibrary.PrintString` "Water" true true (struct :`G` 0.020693 :`B` 0.390625 :`A` 1.0))
        (bind _returnvalue (`|SpawnActorFromClass` "/Game/Elvyn/Blueprints/BP_WaterDrop.BP_WaterDrop_C" (`KismetMathLibrary.MakeTransform` (`SceneComponent.K2_GetComponentLocation` (`self.Arrow_0`)) (struct) (0.1 0.1 0.1)) "Undefined" "OverrideRootScale" null null))
        (`PrimitiveComponent.AddImpulse` (`/Game/Elvyn/Blueprints/BP_WaterDrop.Sphere` _returnvalue) (* (`SceneComponent.GetForwardVector` (`self.Arrow_0`)) (`self.Bullet Velocity_0`)) "None" false)))))

(event `Key|E`
  (params (Key :type "Key Structure"))
  ;[1 1 1] switch weapon
  (:`Pressed`
    (bind _return_value (`self.Weapon Check`))
    (if _return_value
      (bind _isa (`/Engine/EditorBlueprintResources/StandardMacros.FlipFlop`)
        (:`A`
          _)
        (:`B`
          _))
      (bind _output_get (set `self.FireMode` _isa))
      (`KismetSystemLibrary.PrintString` (`KismetStringLibrary.Conv_BoolToString` _output_get)))))

(event `self.Cylinder.OnComponentBeginOverlap`
  (params (OverlappedComponent :type "PrimitiveComponent Object Reference") (OtherActor :type "Actor Object Reference") (OtherComp :type "PrimitiveComponent Object Reference") (OtherBodyIndex :type Integer) (bFromSweep :type Boolean) (SweepResult :type "HitResult Structure (by ref)"))
  ;[1 1 1] add to zone
  (bind _return_value (`self.Weapon Check`))
  (if _return_value
    (if (== (`GameplayStatics.GetObjectClass` OtherActor) "/Game/Elvyn/Blueprints/NPC_Nemo.NPC_Nemo_C")
      (bind _asnpc_nemo (cast `/Game/Elvyn/Blueprints/NPC_Nemo` OtherActor))
      (`KismetArrayLibrary.Array_AddUnique` (`self.Hostiles`) _asnpc_nemo))))

(event `self.Cylinder.OnComponentEndOverlap`
  (params (OverlappedComponent :type "PrimitiveComponent Object Reference") (OtherActor :type "Actor Object Reference") (OtherComp :type "PrimitiveComponent Object Reference") (OtherBodyIndex :type Integer))
  ;[1 1 1] remove from zone
  (bind _asnpc_nemo (cast `/Game/Elvyn/Blueprints/NPC_Nemo` OtherActor))
  (`KismetArrayLibrary.Array_RemoveItem` (`self.Hostiles`) _asnpc_nemo))

(fn `UserConstructionScript`)

(fn `Weapon Check`
  (returns (`Return value` :type Boolean))
  (bind _asfirst_person_character (cast `/Game/FirstPersonBP/Blueprints/FirstPersonCharacter` (`GameplayStatics.GetPlayerPawn` 0)))
  (return (== (`/Game/FirstPersonBP/Blueprints/FirstPersonCharacter.WeaponEquipedIndex` _asfirst_person_character) 1)))