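; BP_MainWeapon is a weapon actor whose Shoot event fires from the player's camera view.
; Shoot prints a debug message, then line traces 5000 units along the first player camera manager's forward vector on the Visibility channel.
; On a hit, it spawns a FirstPersonProjectile at the impact point rather than launching one from the weapon.
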(event `Shoot`
  (bind _returnvalue (`GameplayStatics.GetPlayerCameraManager` 0))
  (bind _returnvalue_2 (`self.K2_GetActorLocation` _returnvalue))
  (`KismetSystemLibrary.PrintString` "Shoot")
  (bind (_outhit _returnvalue_3) (`KismetSystemLibrary.LineTraceSingle` _returnvalue_2 (+ _returnvalue_2 (* (`self.GetActorForwardVector` _returnvalue) 5000.0)) "TraceTypeQuery1"))
  (if _returnvalue_3
    (`|SpawnActorFromClass` "/Game/FirstPersonBP/Blueprints/FirstPersonProjectile.FirstPersonProjectile_C" (`KismetMathLibrary.Conv_VectorToTransform` (`.ImpactPoint` (`GameplayStatics.BreakHitResult` _outhit))) "Undefined" "OverrideRootScale" null null)))

(fn `UserConstructionScript`)