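; BP_BA-RPP_999 is a water and ice gun that fires on a looping timer while the right mouse button is held.
; The game mode's FireMode selects between launching short-lived BP_WaterDrop projectiles and icing wet NPC_Nemo targets; dry ones only print "slowed".
; A cone overlap maintains the ice target list and recolors NPCs entering or leaving it.
; The weapon-index check and local FireMode toggle are unconnected.
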(event `self.ReceiveBeginPlay`
  (`self.EnableInput` (`GameplayStatics.GetPlayerController` 0))
  (`KismetSystemLibrary.K2_SetTimerDelegate` (delegate `UseGun`) 0.1 true))

(event `UseGun`
  (if (`self.Left Mouse Held`)
    (bind _asbp_main_game_mode (cast `/Game/Elvyn/Blueprints/BP_MainGamemode` (`GameplayStatics.GetGameMode`)))
    (if (`/Game/Elvyn/Blueprints/BP_MainGamemode.FireMode` _asbp_main_game_mode)
      ;[1 1 1] Ice
      (`KismetSystemLibrary.PrintString` "ice")
      (for _array_element (`self.Hostiles`)
        (bind _asnpc_nemo (cast `/Game/Elvyn/Blueprints/NPC_Nemo` _array_element))
        (if (`/Game/Elvyn/Blueprints/NPC_Nemo.Wet` _asnpc_nemo)
          (set `/Game/Elvyn/Blueprints/NPC_Nemo.Iced` true _asnpc_nemo)
          (`KismetSystemLibrary.PrintString` "iced")
          (else
            (`KismetSystemLibrary.PrintString` "slowed"))))
      (else
        ;[1 1 1] Water
        (`KismetSystemLibrary.PrintString` "water")
        (bind _returnvalue (`|SpawnActorFromClass` "/Game/Elvyn/Blueprints/BP_WaterDrop.BP_WaterDrop_C" (`KismetMathLibrary.MakeTransform` (`SceneComponent.K2_GetComponentLocation` (`self.Arrow`)) (struct) (0.1 0.1 0.1)) "Undefined" "OverrideRootScale" null null))
        (`PrimitiveComponent.AddImpulse` (`/Game/Elvyn/Blueprints/BP_WaterDrop.Sphere` _returnvalue) (* (`SceneComponent.GetForwardVector` (`self.Arrow`)) (`self.Bullet Velocity`)) "None" true)
        (`KismetSystemLibrary.Delay` 3.0)
        (`self.K2_DestroyActor` _returnvalue)))))

(event `Key|RightMouseButton`
  (params (Key :type "Key Structure"))
  (:`Pressed`
    (set `self.Left Mouse Held` true))
  (:`Released`
    (set `self.Left Mouse Held` false)))

(event `Key|E`
  (params (Key :type "Key Structure")))

(event `self.Cone.OnComponentBeginOverlap`
  (params (OverlappedComponent :type "PrimitiveComponent Object Reference") (OtherActor :type "Actor Object Reference") (OtherComp :type "PrimitiveComponent Object Reference") (OtherBodyIndex :type Integer) (bFromSweep :type Boolean) (SweepResult :type "HitResult Structure (by ref)"))
  ;[1 1 1] Add unique npc to table when in cone
  (if (== (`GameplayStatics.GetObjectClass` OtherActor) "/Game/Elvyn/Blueprints/NPC_Nemo.NPC_Nemo_C")
    (bind _asnpc_nemo (cast `/Game/Elvyn/Blueprints/NPC_Nemo` OtherActor))
    (`KismetArrayLibrary.Array_AddUnique` (`self.Hostiles`) _asnpc_nemo)
    (bind _returnvalue (`self.GetComponentByClass` _asnpc_nemo "/Script/Engine.SkeletalMeshComponent"))
    ;[1 1 1] color when in cone
    (bind _returnvalue_2 (`PrimitiveComponent.CreateDynamicMaterialInstance` _returnvalue 0 (`PrimitiveComponent.GetMaterial` _returnvalue 0) "None"))
    (`MaterialInstanceDynamic.SetVectorParameterValue` _returnvalue_2 "BodyColor" (`self.In Color`))))

(event `self.Cone.OnComponentEndOverlap`
  (params (OverlappedComponent :type "PrimitiveComponent Object Reference") (OtherActor :type "Actor Object Reference") (OtherComp :type "PrimitiveComponent Object Reference") (OtherBodyIndex :type Integer))
  ;[1 1 1] remove npc from table when exiting the cone
  (bind _asnpc_nemo (cast `/Game/Elvyn/Blueprints/NPC_Nemo` OtherActor))
  (`KismetArrayLibrary.Array_RemoveItem` (`self.Hostiles`) _asnpc_nemo)
  (bind _returnvalue (`self.GetComponentByClass` _asnpc_nemo "/Script/Engine.SkeletalMeshComponent"))
  ;[1 1 1] color when out of cone
  (bind _returnvalue_2 (`PrimitiveComponent.CreateDynamicMaterialInstance` _returnvalue 0 (`PrimitiveComponent.GetMaterial` _returnvalue 0) "None"))
  (`MaterialInstanceDynamic.SetVectorParameterValue` _returnvalue_2 "BodyColor" (`self.Out Color`)))

(fn `UserConstructionScript`
  (`parent.UserConstructionScript`))

(fn `Weapon Index Check`
  (returns (ReturnValue :type Boolean))
  (bind _asfirst_person_character (cast `/Game/FirstPersonBP/Blueprints/FirstPersonCharacter` (`GameplayStatics.GetPlayerPawn` 0)))
  (return (== (`/Game/FirstPersonBP/Blueprints/FirstPersonCharacter.WeaponEquipedIndex` _asfirst_person_character) 1)))