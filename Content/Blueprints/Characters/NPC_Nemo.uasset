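; NPC_Nemo is an NPC character with health, death and elemental status states.
; StateManager switches on State, calling the add functions for Wet, Slow and Iced effects, or resetting body color to white through a dynamic material for None.
; AnyDamage clamps health and updates the health bar in its widget component.
; At zero health it disables capsule collision, detaches its controller and destroys itself after a delay.
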(event `self.ReceiveBeginPlay`
  (bind _returnvalue (`|CreateWidget` "/Game/Blueprints/Interface/WBP_HealthBar.WBP_HealthBar_C" null self))
  (set `self.HealthBar` _returnvalue))

(event `StateManager`
  (bind _returnvalue (`self.GetComponentByClass` "/Script/Engine.SkeletalMeshComponent"))
  (`KismetSystemLibrary.PrintString` "StateManager call")
  (switch `/Game/Blueprints/Weapons/BA-RPP99/States` (`self.State`)
    (:`NewEnumerator4`
      (bind _returnvalue_2 (`PrimitiveComponent.CreateDynamicMaterialInstance` _returnvalue 0 (`PrimitiveComponent.GetMaterial` _returnvalue 0) "None"))
      (`MaterialInstanceDynamic.SetVectorParameterValue` _returnvalue_2 "BodyColor" (struct :`R` 1.0 :`G` 1.0 :`B` 1.0 :`A` 1.0)))
    (:`NewEnumerator0`
      (`AddComponent|NODE_AddAC_Wet-1`))
    (:`NewEnumerator1`
      (`AddComponent|NODE_AddAC_Slow-0`))
    (:`NewEnumerator2`
      (`AddComponent|NODE_AddAC_Iced-0`))))

(event `self.ReceiveAnyDamage`
  (params (Damage :type "Float (single-precision)") (DamageType :type "DamageType Object Reference") (InstigatedBy :type "Controller Object Reference") (DamageCauser :type "Actor Object Reference"))
  (bind _healthmax (`self.HealthMax`))
  (bind _output_get (set `self.Health` (`KismetMathLibrary.FClamp` (- (`self.Health`) Damage) 0.0 _healthmax)))
  (bind _aswbp_health_bar (cast `/Game/Blueprints/Interface/WBP_HealthBar` (`WidgetComponent.GetUserWidgetObject` (`self.Widget`))))
  (`/Game/Blueprints/Interface/WBP_HealthBar.HealthUpdate` _aswbp_health_bar (/ _output_get _healthmax))
  (if (== _output_get 0.0)
    (set `self.IsDead` true)
    (`PrimitiveComponent.SetCollisionEnabled` (`self.CapsuleComponent`) "NoCollision")
    (`self.DetachFromControllerPendingDestroy`)
    (`KismetSystemLibrary.Delay` 5.0)
    (`self.K2_DestroyActor`)))

(fn `UserConstructionScript`)