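; BP_Electric220 is an electric hitscan weapon with an overheat mechanic.
; Shoot line-traces from the player camera, spawning a hit effect and radial damage that ignores the player, and adds heat.
; Tick cools the weapon and dispatches the heat percentage; reaching maximum heat blocks firing until heat returns to zero.
; BeginPlay creates the overheat HUD widget, while the shield spawning and overheat alarm logic in the EventGraph is unconnected.
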(event `self.ReceiveBeginPlay`
  (`self.EnableInput` (`GameplayStatics.GetPlayerController` 0))
  (bind _returnvalue (`|CreateWidget` "/Game/Blueprints/Interface/OverHeat_HUD.OverHeat_HUD_C" null self))
  (set `self.Widget` _returnvalue))

(event `self.Shoot`
  (bind _returnvalue (`GameplayStatics.GetPlayerCameraManager` 0))
  (bind _returnvalue_2 (`self.K2_GetActorLocation` _returnvalue))
  (if (not (`self.WeaponOverheated`))
    (`self.ElectricShoot` _returnvalue_2 (+ _returnvalue_2 (* (`self.GetActorForwardVector` _returnvalue) (`self.ShootDisanceMax`))))
    (`self.FireHeat Build Up`)
    (set `self.Shot` true)))

(event `Key|RightMouseButton`
  (params (Key :type "Key Structure")))

(event `self.ReceiveTick`
  (params (DeltaSeconds :type "Float (single-precision)"))
  (`self.Reduce Heat Build Up` DeltaSeconds))

(fn `CheckIfShieldIsDead`
  (if (<= (`self.ref_LifeOfShield`) 0.0)
    (set `self.isShieldReloading` false)))

(fn `ElectricShoot`
  (params (`Start Location` :type "Vector Structure") (`End Location` :type "Vector Structure"))
  (`KismetArrayLibrary.Array_AddUnique` (`self.Ignore Actors`) (`GameplayStatics.GetPlayerCharacter` 0))
  (bind (_outhit _returnvalue) (`KismetSystemLibrary.LineTraceSingle` :`Start` `Start Location` :`End` `End Location` :`TraceChannel` "TraceTypeQuery1" :`DrawDebugType` "Persistent"))
  (if _returnvalue
    (bind (_bblockinghit _binitialoverlap _time _distance _location) (`GameplayStatics.BreakHitResult` _outhit))
    (`GameplayStatics.SpawnEmitterAtLocation` "/Game/FXVarietyPack/Particles/P_ky_hit2.P_ky_hit2" _location)
    (`GameplayStatics.ApplyRadialDamage` 10.0 _location 500.0 null (`self.Ignore Actors`) null null)))

(fn `FireHeat Build Up`
  (bind _returnvalue (+ (`self.HeatCurrent`) (`self.HeatBuildUpRate`)))
  (if (>= _returnvalue (`self.HeatMax`))
    (set `self.HeatCurrent` (`self.HeatMax`))
    (bind _output_get (set `self.WeaponOverheated` true))
    (`self.WeaponOverheatedDispatcher` _output_get)
    (else
      (set `self.HeatCurrent` _returnvalue))))

(fn `Reduce Heat Build Up`
  (params (`Delta T` :type "Float (double-precision)"))
  (bind _returnvalue (- (`self.HeatCurrent`) (* `Delta T` (`self.HeatReductionRate`))))
  (`|ExecutionSequence`
    (:`then_0`
      (if (> (`self.HeatCurrent`) 0.0)
        (if (<= _returnvalue 0.0)
          (set `self.HeatCurrent` 0.0)
          (bind _output_get (set `self.WeaponOverheated` false))
          (`self.WeaponOverheatedDispatcher` _output_get)
          (else
            (set `self.HeatCurrent` _returnvalue)))))
    (:`then_1`
      (`self.WeaponOverheatPercentDispatcher` (/ (`self.HeatCurrent`) (`self.HeatMax`))))))

(fn `UpdateLifeOfShield`
  (returns (ShieldLife :type "Float (double-precision)"))
  (bind _ref_shield (`self.ref_Shield`))
  (`/Engine/EditorBlueprintResources/StandardMacros.IsValid` _ref_shield
    (:`Is Valid`
      (bind _output_get (set `self.ref_LifeOfShield` (`/Game/Blueprints/Weapons/Electric220/BP_Shield.Life Of Shield` _ref_shield)))
      (return _output_get))))

(fn `UserConstructionScript`
  (`parent.UserConstructionScript`))