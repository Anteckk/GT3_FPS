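; Mine launcher weapon that fires physical BP_Mine actors with a cooldown between shots.
; On BeginPlay it enables player input and creates a WBP_Mine_Launcher widget holding a reference to itself.
; Shoot spawns a scaled-down mine at the arrow component and launches it forward with a velocity-change impulse.
; It also counts shots, sets a Shot flag and gates refiring through CanShoot and a Delay.
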(event `self.ReceiveBeginPlay`
  (`self.EnableInput` (`GameplayStatics.GetPlayerController` 0))
  (bind _returnvalue (`|CreateWidget` "/Game/Blueprints/Interface/WBP_Mine_Launcher.WBP_Mine_Launcher_C" null self))
  (set `self.Widget` _returnvalue))

(event `self.Shoot`
  (if (`self.CanShoot`)
    (`/Engine/EditorBlueprintResources/StandardMacros.IncrementInt` (`self.NBShots`)
      (:`  `
        (bind _returnvalue (`|SpawnActorFromClass` "/Game/Blueprints/Weapons/MineLauncher/BP_Mine.BP_Mine_C" (`KismetMathLibrary.MakeTransform` (`SceneComponent.K2_GetComponentLocation` (`self.Arrow_0`)) (struct) (0.2 0.2 0.2)) "Undefined" "OverrideRootScale" null null))
        (`PrimitiveComponent.AddImpulse` (`/Game/Blueprints/Weapons/MineLauncher/BP_Mine.Mine` _returnvalue) (* (`SceneComponent.GetForwardVector` (`self.Arrow_0`)) 1200.0) "None" true)
        (set `self.CanShoot` false)
        (set `self.Shot` true)
        (`KismetSystemLibrary.Delay` 1.5)
        (set `self.CanShoot` true)))))

(fn `UserConstructionScript`
  (`parent.UserConstructionScript`))