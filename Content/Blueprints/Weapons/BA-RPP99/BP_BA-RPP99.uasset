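; BA-RPP99 player weapon with a water mode and an ice mode, toggled with E and active only while weapon slot 1 is equipped.
; Water mode launches a BP_WaterDrop by physics impulse from the Arrow.
; Ice mode flashes a Cylinder and drives state changes on overlap-tracked NPC_Nemo enemies, icing wet ones and slowing the rest.
; A looping timer regenerates ammo, with a CanShoot flag intended as an empty-magazine cooldown.
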(event `self.ReceiveBeginPlay`
  ;[1 1 1] Enabling input, setting auto fire rate and setting the Widget class
  (`self.EnableInput` (`GameplayStatics.GetPlayerController` 0))
  (bind _returnvalue (`|CreateWidget` "/Game/Blueprints/Interface/WBP_BA-RPP_99.WBP_BA-RPP_99_C" null null null self))
  (set `self.Widget` _returnvalue)
  (`KismetSystemLibrary.K2_SetTimerDelegate` (delegate `reload`) 0.5 true)
  (set `self.FireRate` 0.1))

(event `reload`
  (bind _numberofbullets (`self.NumberOfBullets`))
  (bind _numberofbullets_2 (`self.NumberOfBullets`))
  ;[1 1 1] Ammo cooldown
  ;;[1 1 1] add ammo over time
  (if (not (== _numberofbullets_2 (`self.MaxBullet`)))
    (set `self.NumberOfBullets` (`KismetMathLibrary.Clamp` (+ _numberofbullets_2 2) 0 (`self.MaxBullet`)))
    ;;[1 1 1] condition for reloading
    (if (<= _numberofbullets 0)
      (set `self.Can shoot` false)
      (elif (== _numberofbullets (`self.MaxBullet`))
        (set `self.Can shoot` true)))))

(event `self.Shoot`
  (bind _cylinder (`self.Cylinder`))
  ;[1 1 1] START
  ;[1 1 1] Weapon check To shoot
  (bind _return_value (`self.Weapon Check`))
  (if _return_value
    ;[1 1 1] check if he can shoot because of the cooldown from 0
    (if (`self.Can shoot`)
      ;[1 1 1] Subract 1 to the ammo count
      (`/Engine/EditorBlueprintResources/StandardMacros.DecrementInt` (`self.NumberOfBullets`)
        (:`  `
          ;[1 1 1] check fire mode
          (if (`self.FireMode`)
            (`SceneComponent.SetVisibility` _cylinder true false)
            (`KismetSystemLibrary.Delay` 0.2)
            (`SceneComponent.SetVisibility` _cylinder false false)
            ;[1 1 1] Ice/ slow mode
            (for _array_element (`self.Hostiles`)
              (if (`/Game/Blueprints/Characters/NPC_Nemo.Wet` _array_element)
                (if (`/Game/Blueprints/Characters/NPC_Nemo.Iced` _array_element)
                  (`KismetSystemLibrary.PrintString` "alreadt iced")
                  (else
                    (set `/Game/Blueprints/Characters/NPC_Nemo.Iced` true _array_element)
                    (set `/Game/Blueprints/Characters/NPC_Nemo.State` "NewEnumerator2" _array_element)
                    (`/Game/Blueprints/Characters/NPC_Nemo.StateManager` _array_element)))
                (elif (`/Game/Blueprints/Characters/NPC_Nemo.Slowed` _array_element)
                  (`KismetSystemLibrary.PrintString` "already slowed")
                  (else
                    (set `/Game/Blueprints/Characters/NPC_Nemo.Slowed` true _array_element)
                    (set `/Game/Blueprints/Characters/NPC_Nemo.State` "NewEnumerator1" _array_element)
                    (`/Game/Blueprints/Characters/NPC_Nemo.StateManager` _array_element)))))
            (else
              ;[1 1 1] water mode
              (bind _returnvalue (`|SpawnActorFromClass` "/Game/Blueprints/Weapons/BA-RPP99/BP_WaterDrop.BP_WaterDrop_C" (`KismetMathLibrary.MakeTransform` (`SceneComponent.K2_GetComponentLocation` (`self.Arrow`)) (struct) (0.1 0.1 0.1)) "Undefined" "OverrideRootScale" null null))
              (`/Engine/EditorBlueprintResources/StandardMacros.IsValid` _returnvalue
                (:`Is Valid`
                  (`PrimitiveComponent.AddImpulse` (`/Game/Blueprints/Weapons/BA-RPP99/BP_WaterDrop.Sphere` _returnvalue) (* (`SceneComponent.GetForwardVector` (`self.Arrow`)) (`self.Bullet Velocity_0`)) "None" false)
                  (set `self.Shot` true))))))))))

(event `Key|E`
  (params (Key :type "Key Structure"))
  ;[1 1 1] switch weapon
  (:`Pressed`
    (bind _return_value (`self.Weapon Check`))
    (if _return_value
      (bind _isa (`/Engine/EditorBlueprintResources/StandardMacros.FlipFlop`)
        (:`A`
          _)
        (:`B`
          _))
      (set `self.FireMode` _isa))))

(event `self.Cylinder.OnComponentBeginOverlap`
  (params (OverlappedComponent :type "PrimitiveComponent Object Reference") (OtherActor :type "Actor Object Reference") (OtherComp :type "PrimitiveComponent Object Reference") (OtherBodyIndex :type Integer) (bFromSweep :type Boolean) (SweepResult :type "HitResult Structure (by ref)"))
  ;[1 1 1] add to zone
  (bind _return_value (`self.Weapon Check`))
  (if _return_value
    (if (`self.ActorHasTag` OtherActor "Enemy")
      (bind _asnpc_nemo (cast `/Game/Blueprints/Characters/NPC_Nemo` OtherActor))
      (`KismetArrayLibrary.Array_AddUnique` (`self.Hostiles`) _asnpc_nemo))))

(event `self.Cylinder.OnComponentEndOverlap`
  (params (OverlappedComponent :type "PrimitiveComponent Object Reference") (OtherActor :type "Actor Object Reference") (OtherComp :type "PrimitiveComponent Object Reference") (OtherBodyIndex :type Integer))
  ;[1 1 1] remove from zone
  (bind _asnpc_nemo (cast `/Game/Blueprints/Characters/NPC_Nemo` OtherActor))
  (`KismetArrayLibrary.Array_RemoveItem` (`self.Hostiles`) _asnpc_nemo))

(fn `UserConstructionScript`)

(fn `Weapon Check`
  (returns (`Return value` :type Boolean))
  (bind _asfirst_person_character (cast `/Game/Blueprints/Characters/FirstPersonCharacter` (`GameplayStatics.GetPlayerPawn` 0)))
  (return (== (`/Game/Blueprints/Characters/FirstPersonCharacter.WeaponEquipedIndex` _asfirst_person_character) 1)))