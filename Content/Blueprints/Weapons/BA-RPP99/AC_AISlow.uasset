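; AC_AISlow is an actor component in the BA-RPP99 weapon folder that periodically slows its owning character and tints its body.
; On BeginPlay it creates a dynamic material on the owner's skeletal mesh, applies the slow immediately, then repeats it on a looping EffectDuration timer.
; Each slow divides MaxWalkSpeed by AccFactor and sets BodyColor to SlowColor, then multiplies speed back and sets DefaultColor after a fixed three-second delay.
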(event `self.ReceiveBeginPlay`
  (bind _returnvalue (`Actor.GetComponentByClass` (`self.GetOwner`) "/Script/Engine.SkeletalMeshComponent"))
  (bind _returnvalue_2 (`PrimitiveComponent.CreateDynamicMaterialInstance` _returnvalue 0 (`PrimitiveComponent.GetMaterial` _returnvalue 0) "None"))
  (set `self.Material Instance` _returnvalue_2)
  (`self.Slow`)
  (`KismetSystemLibrary.K2_SetTimerDelegate` (delegate `Slow`) (`self.Effect Duration`) true))

(event `Slow`
  (bind _returnvalue (`Actor.GetComponentByClass` (`self.GetOwner`) "/Script/Engine.CharacterMovementComponent"))
  (bind _output_get (set `CharacterMovementComponent.MaxWalkSpeed` (/ (`CharacterMovementComponent.MaxWalkSpeed` _returnvalue) (`self.Acc Factor`)) _returnvalue))
  (`MaterialInstanceDynamic.SetVectorParameterValue` (`self.Material Instance`) "BodyColor" (`self.Slow Color`))
  (`KismetSystemLibrary.Delay` 3.0)
  (set `CharacterMovementComponent.MaxWalkSpeed` (* _output_get (`self.Acc Factor`)) _returnvalue)
  (`MaterialInstanceDynamic.SetVectorParameterValue` (`self.Material Instance`) "BodyColor" (`self.Default Color`)))