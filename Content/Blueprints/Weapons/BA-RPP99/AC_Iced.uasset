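; AC_Iced is an actor component that applies a temporary freeze to its owning NPC_Nemo, likely attached by the BA-RPP99 weapon.
; On BeginPlay it deactivates the NPC's character movement for a fixed delay, printing a debug message.
; It then reactivates movement, clears the Iced flag, sets a new state through StateManager, and destroys itself.
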(event `self.ReceiveBeginPlay`
  (bind _asnpc_nemo (cast `/Game/Blueprints/Characters/NPC_Nemo` (`self.GetOwner`)))
  (`KismetSystemLibrary.PrintString` "Iced")
  (bind _charactermovement (`Character.CharacterMovement` _asnpc_nemo))
  (`self.Deactivate` _charactermovement)
  (`KismetSystemLibrary.Delay` 5.0)
  (`self.Activate` _charactermovement false)
  (set `/Game/Blueprints/Characters/NPC_Nemo.Iced` false _asnpc_nemo)
  (set `/Game/Blueprints/Characters/NPC_Nemo.State` "NewEnumerator4" _asnpc_nemo)
  (`/Game/Blueprints/Characters/NPC_Nemo.StateManager` _asnpc_nemo)
  (`self.K2_DestroyComponent`))