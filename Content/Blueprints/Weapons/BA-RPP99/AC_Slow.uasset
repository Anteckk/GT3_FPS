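; AC_Slow is an actor component in the BA-RPP99 weapon folder that temporarily slows the NPC_Nemo it is attached to.
; On BeginPlay it divides the owner's max walk speed by that NPC's SlowFactor and waits five seconds.
; It then multiplies the speed back, sets the NPC's state, runs its StateManager and destroys itself.
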(event `self.ReceiveBeginPlay`
  (bind _asnpc_nemo (cast `/Game/Blueprints/Characters/NPC_Nemo` (`self.GetOwner`)))
  (bind _charactermovement (`Character.CharacterMovement` _asnpc_nemo))
  (bind _maxwalkspeed (`CharacterMovementComponent.MaxWalkSpeed` _charactermovement))
  (bind _slowfactor (`/Game/Blueprints/Characters/NPC_Nemo.SlowFactor` _asnpc_nemo))
  (set `CharacterMovementComponent.MaxWalkSpeed` (/ _maxwalkspeed _slowfactor) _charactermovement)
  (`KismetSystemLibrary.Delay` 5.0)
  (set `CharacterMovementComponent.MaxWalkSpeed` (* _maxwalkspeed _slowfactor) _charactermovement)
  (set `/Game/Blueprints/Characters/NPC_Nemo.State` "NewEnumerator4" _asnpc_nemo)
  (`/Game/Blueprints/Characters/NPC_Nemo.StateManager` _asnpc_nemo)
  (`self.K2_DestroyComponent`))