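; BP_WaterDrop is a short-lived water drop for the BA-RPP99 weapon that destroys itself after three seconds.
; Overlapping an Enemy-tagged NPC_Nemo marks it wet, updates its state, knocks it horizontally away from the player and applies environmental damage.
; A successful enemy hit or an overlap with a Floor-tagged actor spawns a water-ball hit particle and destroys the drop.
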(event `self.ReceiveBeginPlay`
  ;[1 1 1] auto destroy after 3 sec
  (`KismetSystemLibrary.Delay` 3.0)
  (`/Engine/EditorBlueprintResources/StandardMacros.IsValid` self
    (:`Is Valid`
      (`self.K2_DestroyActor`))))

(event `self.Sphere1.OnComponentBeginOverlap`
  (params (OverlappedComponent :type "PrimitiveComponent Object Reference") (OtherActor :type "Actor Object Reference") (OtherComp :type "PrimitiveComponent Object Reference") (OtherBodyIndex :type Integer) (bFromSweep :type Boolean) (SweepResult :type "HitResult Structure (by ref)"))
  (if (`self.ActorHasTag` OtherActor "Enemy")
    (bind _asnpc_nemo (cast `/Game/Blueprints/Characters/NPC_Nemo` OtherActor))
    (set `/Game/Blueprints/Characters/NPC_Nemo.Wet` true _asnpc_nemo)
    (set `/Game/Blueprints/Characters/NPC_Nemo.State` "NewEnumerator0" _asnpc_nemo)
    (`/Game/Blueprints/Characters/NPC_Nemo.StateManager` _asnpc_nemo)
    (bind (_returnvalue_x _returnvalue_y) (`KismetMathLibrary.BreakVector` (* (`KismetMathLibrary.GetDirectionUnitVector` (`self.K2_GetActorLocation` (`GameplayStatics.GetPlayerPawn` 0)) (`self.K2_GetActorLocation` _asnpc_nemo)) (`self.KnockBack Force`))))
    (`Character.LaunchCharacter` _asnpc_nemo (`KismetMathLibrary.MakeVector` _returnvalue_x _returnvalue_y) true false)
    (`/Engine/EditorBlueprintResources/StandardMacros.IsValid` self
      (:`Is Valid`
        (`GameplayStatics.ApplyDamage` _asnpc_nemo 10.0 null self "/Engine/EngineDamageTypes/DmgTypeBP_Environmental.DmgTypeBP_Environmental_C")
        (`/Engine/EditorBlueprintResources/StandardMacros.IsValid` self
          (:`Is Valid`
            (`GameplayStatics.SpawnEmitterAtLocation` "/Game/FXVarietyPack/Particles/P_ky_waterBallHit.P_ky_waterBallHit" (`self.K2_GetActorLocation` self) (struct) (0.5 0.5 0.5) :!label _label)
            (`self.K2_DestroyActor`)))))
    (elif (`self.ActorHasTag` OtherActor "Floor")
      (goto _label))))

(fn `UserConstructionScript`)