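; BP_MainWeapon is a weapon actor that fires physical projectiles.
; On BeginPlay it creates and stores a WBP_MainWeapon widget that references the weapon, without adding it to the viewport here.
; Shoot counts the shot, spawns a scaled-down BP_Bullet at the Arrow component and launches its Sphere with an impulse along the arrow's forward vector.
; An unconnected camera-aimed line trace with hit particles remains unused.
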(event `self.ReceiveBeginPlay`
  (bind _returnvalue (`|CreateWidget` "/Game/Blueprints/Interface/WBP_MainWeapon.WBP_MainWeapon_C" null self))
  (set `self.Widget` _returnvalue)
  (cast `/Game/Blueprints/Characters/FirstPersonCharacter` (`GameplayStatics.GetPlayerCharacter` 0)))

(event `Shoot`
  (`/Engine/EditorBlueprintResources/StandardMacros.IncrementInt` (`self.Number of bullets shot`)
    (:`  `
      (bind _returnvalue (`|SpawnActorFromClass` "/Game/Blueprints/Weapons/MainWeapon/BP_Bullet.BP_Bullet_C" (`KismetMathLibrary.MakeTransform` (`SceneComponent.K2_GetComponentLocation` (`self.Arrow`)) (struct) (0.1 0.1 0.1)) "Undefined" "OverrideRootScale" null null))
      (bind _sphere (`/Game/Blueprints/Weapons/MainWeapon/BP_Bullet.Sphere` _returnvalue))
      (`/Engine/EditorBlueprintResources/StandardMacros.IsValid` _sphere
        (:`Is Valid`
          (`PrimitiveComponent.AddImpulse` _sphere (* (`SceneComponent.GetForwardVector` (`self.Arrow`)) (`self.Bullet Velocity`)) "None" false)
          (set `self.Shot` true))))))

(fn `UserConstructionScript`)