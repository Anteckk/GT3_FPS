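; BP_BA-RPP_99 is a shootable child Blueprint whose cone applies a freeze effect to wet NPC_Nemo characters.
; Shoot calls the parent implementation and prints the asset name as debug output.
; Cone overlap casts to NPC_Nemo and, if Wet, sets Iced for five seconds using a Delay.
; Dry targets only trigger a "slowed" debug print, with no actual slowdown applied.
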(event `self.Shoot`
  (`parent.Shoot`)
  (`KismetSystemLibrary.PrintString` "BP_BA-RPP_99"))

(event `Key|LeftMouseButton`
  (params (Key :type "Key Structure")))

(event `self.Cone.OnComponentBeginOverlap`
  (params (OverlappedComponent :type "PrimitiveComponent Object Reference") (OtherActor :type "Actor Object Reference") (OtherComp :type "PrimitiveComponent Object Reference") (OtherBodyIndex :type Integer) (bFromSweep :type Boolean) (SweepResult :type "HitResult Structure (by ref)"))
  (bind _asnpc_nemo (cast `/Game/Elvyn/Blueprints/NPC_Nemo` OtherActor))
  (if (`/Game/Elvyn/Blueprints/NPC_Nemo.Wet` _asnpc_nemo)
    (set `/Game/Elvyn/Blueprints/NPC_Nemo.Iced` true _asnpc_nemo)
    (`KismetSystemLibrary.Delay` 5.0)
    (set `/Game/Elvyn/Blueprints/NPC_Nemo.Iced` false _asnpc_nemo)
    (elif true
      (`KismetSystemLibrary.PrintString` "slowed"))))

(fn `UserConstructionScript`
  (`parent.UserConstructionScript`))