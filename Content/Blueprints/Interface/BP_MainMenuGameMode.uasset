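; Main menu game mode Blueprint, by name, that holds checkpoint, game-over and weapon fire-mode logic.
; UpdateCheckpoint stores and prints the latest checkpoint, while GameOver prints a message, waits briefly and opens the ElvynSalle level.
; The E key flips FireMode through a FlipFlop when the player's equipped weapon index is 1.
; BeginPlay is empty, leaving the player lookup and EnableInput nodes disconnected.
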(event `self.ReceiveBeginPlay`
  ;[1 1 1] Gets the player character
)

(event `Update Checkpoint`
  (params (newCheckPoint :type "Transform Structure"))
  ;[1 1 1] Update and prints location of checkpoint
  (bind _output_get (set `self.lastCheckPoint` newCheckPoint))
  (`KismetSystemLibrary.PrintString` (`KismetStringLibrary.Conv_TransformToString` _output_get)))

(event `GameOver`
  ;[1 1 1] Prints Gameover and opens the level
  (`KismetSystemLibrary.PrintString` "Game over")
  (`KismetSystemLibrary.Delay` 2.0)
  (`GameplayStatics.OpenLevelBySoftObjectPtr` "/Game/Blueprints/Levels/ElvynSalle.ElvynSalle"))

(event `Key|E`
  (params (Key :type "Key Structure"))
  ;[1 1 1] Switch for weapon Mode
  (:`Pressed`
    (bind _returnvalue (`self.Check Weapon Index`))
    (if _returnvalue
      (bind _isa (`/Engine/EditorBlueprintResources/StandardMacros.FlipFlop`)
        (:`A`
          _)
        (:`B`
          _))
      (set `self.FireMode` _isa)
      (`KismetSystemLibrary.PrintString` (`KismetStringLibrary.Conv_BoolToString` (`self.FireMode`))))))

(fn `Check Weapon Index`
  (returns (ReturnValue :type Boolean))
  (bind _asfirst_person_character (cast `/Game/Blueprints/Characters/FirstPersonCharacter` (`GameplayStatics.GetPlayerPawn` 0)))
  (return (== (`/Game/Blueprints/Characters/FirstPersonCharacter.WeaponEquipedIndex` _asfirst_person_character) 1)))

(fn `UserConstructionScript`)